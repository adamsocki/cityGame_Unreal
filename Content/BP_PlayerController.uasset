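; Player controller that drives the camera character and triggers building placement from mouse input.
; Movement, zoom and pitch inputs cast the controlled pawn to BP_CameraCharacter and forward to its camera functions.
; Holding right mouse sets a flag on InputController that gates mouse-driven orbit and pitch.
; Left click calls SpawnBuilding on PlacementController while placement mode is enabled; the UpdatePlacement branch is unconnected and Tick is empty.
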(event `InputAxis|MovementForward/Backward`
  (params (AxisValue :type "Float (single-precision)"))
  (bind _asbp_camera_character (cast `/Game/BP_CameraCharacter` (`self.K2_GetPawn`)))
  (`/Game/BP_CameraCharacter.CameraForwardBackward` _asbp_camera_character AxisValue))

(event `InputAxis|MovementLeft/Right`
  (params (AxisValue :type "Float (single-precision)"))
  (bind _asbp_camera_character (cast `/Game/BP_CameraCharacter` (`self.K2_GetPawn`)))
  (`/Game/BP_CameraCharacter.CameraLeftRight` _asbp_camera_character AxisValue))

(event `InputAction|CameraZoomIn`
  (params (Key :type "Key Structure"))
  (:`Pressed`
    (bind _asbp_camera_character (cast `/Game/BP_CameraCharacter` (`self.K2_GetPawn`)))
    (`/Game/BP_CameraCharacter.CameraZoomIn` _asbp_camera_character 1.0)))

(event `InputAction|CameraZoomOut`
  (params (Key :type "Key Structure"))
  (:`Pressed`
    (bind _asbp_camera_character (cast `/Game/BP_CameraCharacter` (`self.K2_GetPawn`)))
    (`/Game/BP_CameraCharacter.CameraZoomOut` _asbp_camera_character 1.0)))

(event `InputAxis|CameraPitch`
  (params (AxisValue :type "Float (single-precision)"))
  (bind _asbp_camera_character (cast `/Game/BP_CameraCharacter` (`self.K2_GetPawn`)))
  (`/Game/BP_CameraCharacter.CameraPitch` _asbp_camera_character AxisValue))

(event `InputAction|MouseRightClick`
  (params (Key :type "Key Structure"))
  (bind _inputcontroller (`self.InputController`))
  (:`Pressed`
    (set `/Game/InputController.RIghtButtonPressed` true _inputcontroller))
  (:`Released`
    (set `/Game/InputController.RIghtButtonPressed` false _inputcontroller)))

(event `InputAxis|MouseX`
  (params (AxisValue :type "Float (single-precision)"))
  (if (`/Game/InputController.RIghtButtonPressed` (`self.InputController`))
    (bind _asbp_camera_character (cast `/Game/BP_CameraCharacter` (`self.K2_GetPawn`)))
    (`/Game/BP_CameraCharacter.CameraOrbit` _asbp_camera_character AxisValue)))

(event `InputAxis|MouseY`
  (params (AxisValue :type "Float (single-precision)"))
  (if (`/Game/InputController.RIghtButtonPressed` (`self.InputController`))
    (bind _asbp_camera_character (cast `/Game/BP_CameraCharacter` (`self.K2_GetPawn`)))
    (`/Game/BP_CameraCharacter.CameraPitch` _asbp_camera_character AxisValue)))

(event `self.ReceiveTick`
  (params (DeltaSeconds :type "Float (single-precision)")))

(event `Key|LeftMouseButton`
  (params (Key :type "Key Structure"))
  ;[1 1 1] PlacementFunction - BOOL
  (:`Pressed`
    (if (`/Game/PlacementController.PlacementModeEnabled` (`self.PlacementController`))
      (`/Game/PlacementController.SpawnBuilding` (`self.PlacementController`)))))

(fn `UserConstructionScript`)