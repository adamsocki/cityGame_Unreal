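; BP_CameraCharacter is a controllable camera character that supports panning, orbit, pitch and zoom around a spring arm.
; Camera events move the character along the spring arm's forward and right vectors, and orbit through controller yaw input.
; Pitch rotates the spring arm within clamped angles, while zoom changes its arm length without limits.
; MovementComponent supplies the speeds and pitch limits.
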(event `CameraLeftRight`
  (params (Movement :type "Float (double-precision)"))
  (`self.AddMovementInput` (`SceneComponent.GetRightVector` (`self.SpringArm`)) (* Movement (`/Game/MovementComponent.MoveSpeed` (`self.MovementComponent`)))))

(event `CameraForwardBackward`
  (params (Magnitude :type "Float (double-precision)"))
  (`self.AddMovementInput` (`SceneComponent.GetForwardVector` (`self.SpringArm`)) (* Magnitude (`/Game/MovementComponent.MoveSpeed` (`self.MovementComponent`)))))

(event `CameraOrbit`
  (params (Magnitude :type "Float (double-precision)"))
  (`self.AddControllerYawInput` (* Magnitude (`/Game/MovementComponent.OrbitSpeed` (`self.MovementComponent`)))))

(event `CameraPitch`
  (params (Magnitude :type "Float (double-precision)"))
  (bind _movementcomponent (`self.MovementComponent`))
  (`SceneComponent.K2_SetWorldRotation` (`self.SpringArm`) (`KismetMathLibrary.Conv_VectorToRotator` (`KismetMathLibrary.Conv_RotatorToVector` (`KismetMathLibrary.MakeRotator` (.roll (`SceneComponent.K2_GetComponentRotation` (`self.SpringArm`))) (`KismetMathLibrary.ClampAngle` (+ (* (`/Game/MovementComponent.OrbitSpeed` (`self.MovementComponent`)) Magnitude) (.pitch (`SceneComponent.K2_GetComponentRotation` (`self.SpringArm`)))) (`/Game/MovementComponent.ClampAngleMin` _movementcomponent) (`/Game/MovementComponent.ClampAngleMax` _movementcomponent)) (.yaw (`SceneComponent.K2_GetComponentRotation` (`self.SpringArm`)))))) false false))

(event `CameraZoomIn`
  (params (Magnitude :type "Float (double-precision)"))
  (bind _springarm (`self.SpringArm`))
  (set `SpringArmComponent.TargetArmLength` (- (`SpringArmComponent.TargetArmLength` _springarm) (* Magnitude (`/Game/MovementComponent.ZoomSpeed` (`self.MovementComponent`)))) _springarm))

(event `CameraZoomOut`
  (params (Magnitude :type "Float (double-precision)"))
  (bind _springarm (`self.SpringArm`))
  (set `SpringArmComponent.TargetArmLength` (+ (`SpringArmComponent.TargetArmLength` _springarm) (* Magnitude (`/Game/MovementComponent.ZoomSpeed` (`self.MovementComponent`)))) _springarm))

(fn `UserConstructionScript`)